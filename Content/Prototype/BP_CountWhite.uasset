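; Prototype Blueprint that measures a difference percentage and score by counting bright pixels in a render target, triggered by a test event.
; CalculateDifferencesValue draws a subtraction material into the render target, then reads every pixel on the CPU in nested loops, counting those whose red channel meets a threshold.
; It converts the count into a percentage of the texture area, derives a score penalized by that percentage, then prints and returns all three.
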(event `test`
  (`self.Calculate Differences Value` 5.0 "/Game/Prototype/M_SubtractMaterial.M_SubtractMaterial"))

(fn `Calculate Differences Value`
  (params (Tresshold :type "Float (double-precision)" :default 5.0) (`Difference Material` :type "MaterialInterface Object Reference"))
  (returns (`Difference Value` :type "Float (double-precision)") (`Difference Percent` :type "Float (double-precision)") (Score :type "Float (double-precision)"))
  (locals (DifferenceValue :type "Float (double-precision)"))
  (bind _differencevalue (`local.DifferenceValue`))
  (bind _render_target_to_draw (`self.Render Target to Draw`))
  (bind _sizex (`TextureRenderTarget2D.SizeX` _render_target_to_draw))
  (bind _sizey (`TextureRenderTarget2D.SizeY` _render_target_to_draw))
  (bind _returnvalue (* (/ _differencevalue (* _sizex _sizey)) 100.0))
  (bind _returnvalue_2 (- 100.0 (* _returnvalue 1.5)))
  (`KismetRenderingLibrary.DrawMaterialToRenderTarget` (`self.Render Target to Draw`) `Difference Material`)
  (set `local.DifferenceValue` 0.0)
  (for _index (range (+ _sizex 1))
    (for _index_2 (range (+ _sizey 1))
      (bind _returnvalue_3 (`KismetRenderingLibrary.ReadRenderTargetRawPixel` (`self.Render Target to Draw`) _index _index_2))
      (if (>= (`.R` (break `LinearColor` _returnvalue_3)) Tresshold)
        (`/Engine/EditorBlueprintResources/StandardMacros.IncrementFloat` (`local.DifferenceValue`)))))
  (`KismetSystemLibrary.PrintString` (`KismetStringLibrary.Concat_StrStr` "Difference Value " (`KismetStringLibrary.Conv_DoubleToString` _differencevalue) " | " (`KismetStringLibrary.Conv_DoubleToString` _returnvalue) " %" " | " "Score : " (`KismetStringLibrary.Conv_DoubleToString` _returnvalue_2)))
  (return (`local.DifferenceValue`) _returnvalue _returnvalue_2))

(fn `UserConstructionScript`)