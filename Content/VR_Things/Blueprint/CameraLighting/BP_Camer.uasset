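; BP_Camer is a camera actor that animates a SceneCaptureComponent2D along a predefined path of locations and rotations.
; PlayAnimation steps through the Location and Rotator arrays, replaying the Playing timeline to lerp between each pair of keyframes until it reaches the last one.
; Move and Rot snap the capture component to the keyframe at the current Index, while SetCamera is an empty stub.
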(event `Move`
  (`SceneComponent.K2_SetRelativeLocation` (`self.SceneCaptureComponent2D`) (`|GetArrayItem` (`self.Location`) (`self.Index`)) false false))

(event `SetCamera`)

(event `Rot`
  (`SceneComponent.K2_SetRelativeRotation` (`self.SceneCaptureComponent2D`) (`|GetArrayItem` (`self.Rotator`) (`self.Index`)) false false))

(event `PlayAnimation`
  (bind _rotator (`self.Rotator`))
  (bind _index (`self.Index`))
  (bind _scenecapturecomponent2d (`self.SceneCaptureComponent2D`))
  (bind _location (`self.Location`))
  (set `self.Index` 1)
  (if (!= (`self.Index`) (`KismetArrayLibrary.Array_Length` (`self.Location`))) :!label _label
    (bind (_direction _newtrack_0) (`Timeline|Playing` :!via `PlayFromStart`)
      (:`Update`
        (`SceneComponent.K2_SetRelativeLocation` _scenecapturecomponent2d (`KismetMathLibrary.VLerp` (`|GetArrayItem` _location (- _index 1)) (`|GetArrayItem` _location _index) _newtrack_0) false false)
        (`SceneComponent.K2_SetRelativeRotation` _scenecapturecomponent2d (`KismetMathLibrary.RLerp` (`|GetArrayItem` _rotator (- _index 1)) (`|GetArrayItem` _rotator _index) _newtrack_0) false false))
      (:`Finished`
        (`/Engine/EditorBlueprintResources/StandardMacros.IncrementInt` (`self.Index`)
          (:`  `
            (goto _label)))))))

(fn `UserConstructionScript`)