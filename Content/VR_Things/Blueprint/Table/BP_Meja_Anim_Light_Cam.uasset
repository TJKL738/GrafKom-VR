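; VR table that hosts animation, camera and lighting panels as child actors, with buttons pressed by the pawn's index fingers.
; Next and back buttons step OnSegment through the panels, using timelines to lerp them between hidden and ready positions, with input locked during transitions.
; Moving to lighting dims every BP_LampuAll lamp and leaving restores brightness.
; Other buttons play the animation and camera panels together or fire a one-shot CallBackToModelling to switch stage.
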(event `self.ReceiveBeginPlay`
  (bind (_direction _alpha) (`Timeline|Spawn`)
    (:`Update`
      (`self.SwitchPos` null (`self.BP_MejaAnimasi`) _alpha))))

(event `self.SM_Box_2.OnComponentBeginOverlap`
  (params (OverlappedComponent :type "PrimitiveComponent Object Reference") (OtherActor :type "Actor Object Reference") (OtherComp :type "PrimitiveComponent Object Reference") (OtherBodyIndex :type Integer) (bFromSweep :type Boolean) (SweepResult :type "HitResult Structure (by ref)"))
  (bind _onsegment (`self.OnSegment`))
  (`self.CheckJari` OtherActor OtherComp
    (:`Out`
      (if (and (`self.CanReciveInput`) (< (`self.OnSegment`) 2))
        (set `self.CanReciveInput` false)
        (bind (_direction _alpha) (`Timeline|Timeline` :!via `PlayFromStart`)
          (:`Update`
            (if (== _onsegment 0)
              (`self.SwitchPos` (`self.BP_MejaAnimasi`) (`self.BP_MejaCam`) _alpha)
              (elif (== _onsegment 1)
                (`self.SwitchPos` (`self.BP_MejaCam`) (`self.BP_MejaLight`) _alpha
                  (:`Out`
                    (bind _outactors (`GameplayStatics.GetAllActorsOfClass` "/Game/Bulb/BP_LampuAll.BP_LampuAll_C"))
                    (for _array_element _outactors
                      (`/Game/Bulb/BP_LampuAll.SetInten` _array_element 300.0)))))))
          (:`Finished`
            (`/Engine/EditorBlueprintResources/StandardMacros.IncrementInt` (`self.OnSegment`)
              (:`  `
                (set `self.CanReciveInput` true)))))))))

(event `self.SM_Box_3.OnComponentBeginOverlap`
  (params (OverlappedComponent :type "PrimitiveComponent Object Reference") (OtherActor :type "Actor Object Reference") (OtherComp :type "PrimitiveComponent Object Reference") (OtherBodyIndex :type Integer) (bFromSweep :type Boolean) (SweepResult :type "HitResult Structure (by ref)"))
  (bind _onsegment (`self.OnSegment`))
  (`self.CheckJari` OtherActor OtherComp
    (:`Out`
      (if (and (> (`self.OnSegment`) 0) (`self.CanReciveInput`))
        (set `self.CanReciveInput` false)
        (bind (_direction _alpha) (`Timeline|Timeline_0` :!via `PlayFromStart`)
          (:`Update`
            (if (== _onsegment 2)
              (`self.SwitchPos` (`self.BP_MejaLight`) (`self.BP_MejaCam`) _alpha
                (:`Out`
                  (bind _outactors (`GameplayStatics.GetAllActorsOfClass` "/Game/Bulb/BP_LampuAll.BP_LampuAll_C"))
                  (for _array_element _outactors
                    (`/Game/Bulb/BP_LampuAll.SetInten` _array_element 5000.0))))
              (elif (== _onsegment 1)
                (`self.SwitchPos` (`self.BP_MejaCam`) (`self.BP_MejaAnimasi`) _alpha))))
          (:`Finished`
            (`/Engine/EditorBlueprintResources/StandardMacros.DecrementInt` (`self.OnSegment`)
              (:`  `
                (set `self.CanReciveInput` true)))))))))

(event `self.SM_Box_4.OnComponentBeginOverlap`
  (params (OverlappedComponent :type "PrimitiveComponent Object Reference") (OtherActor :type "Actor Object Reference") (OtherComp :type "PrimitiveComponent Object Reference") (OtherBodyIndex :type Integer) (bFromSweep :type Boolean) (SweepResult :type "HitResult Structure (by ref)"))
  (`self.CheckJari` OtherActor OtherComp
    (:`Out`
      (bind _asbp_meja_animasi (cast `/Game/VR_Things/Blueprint/Table/BP_MejaAnimasi` (`ChildActorComponent.ChildActor` (`self.BP_MejaAnimasi`))))
      (bind _asbp_meja_cam (cast `/Game/VR_Things/Blueprint/Table/BP_MejaCam` (`ChildActorComponent.ChildActor` (`self.BP_MejaCam`))))
      (`/Game/VR_Things/Blueprint/Table/BP_MejaAnimasi.PlayAnimation` _asbp_meja_animasi)
      (`/Game/VR_Things/Blueprint/Table/BP_MejaCam.PlayAnimation` _asbp_meja_cam))))

(event `self.Switch Stage Static Mesh.OnComponentBeginOverlap`
  (params (OverlappedComponent :type "PrimitiveComponent Object Reference") (OtherActor :type "Actor Object Reference") (OtherComp :type "PrimitiveComponent Object Reference") (OtherBodyIndex :type Integer) (bFromSweep :type Boolean) (SweepResult :type "HitResult Structure (by ref)"))
  (`self.CheckJari` OtherActor OtherComp
    (:`Out`
      (if (`self.CanPressNext`)
        (set `self.CanPressNext` false)
        (`self.Back to Modelling`)
        (`KismetSystemLibrary.Delay` 1.0)
        (set `self.CanPressNext` false)))))

(fn `UserConstructionScript`)