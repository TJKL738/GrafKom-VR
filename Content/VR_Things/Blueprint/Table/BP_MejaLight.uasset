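; VR control table that spawns, selects, edits and removes BP_Lampu point-light lamps through touch buttons.
; Each static mesh button fires on overlap, filtered by CheckJari to the VRPawnManual's left or right index finger component.
; Buttons choose an axis or RGB channel, then step position, color or intensity on the selected AllLamp entry.
; OnIndex tracks that selection, shown by the PickLampu marker and a text readout.
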(event `self.StaticMesh19.OnComponentBeginOverlap`
  (params (OverlappedComponent :type "PrimitiveComponent Object Reference") (OtherActor :type "Actor Object Reference") (OtherComp :type "PrimitiveComponent Object Reference") (OtherBodyIndex :type Integer) (bFromSweep :type Boolean) (SweepResult :type "HitResult Structure (by ref)"))
  ;[1 1 1] Set Location Type
  (`self.CheckJari` OtherActor OtherComp
    (:`Out`
      (set `self.XYZ` 0))))

(event `self.StaticMesh16.OnComponentBeginOverlap`
  (params (OverlappedComponent :type "PrimitiveComponent Object Reference") (OtherActor :type "Actor Object Reference") (OtherComp :type "PrimitiveComponent Object Reference") (OtherBodyIndex :type Integer) (bFromSweep :type Boolean) (SweepResult :type "HitResult Structure (by ref)"))
  ;[1 1 1] Set Location
  (`self.CheckJari` OtherActor OtherComp
    (:`Out`
      (`self.Location` 20.0 (`self.XYZ`)))))

(event `self.StaticMesh15.OnComponentBeginOverlap`
  (params (OverlappedComponent :type "PrimitiveComponent Object Reference") (OtherActor :type "Actor Object Reference") (OtherComp :type "PrimitiveComponent Object Reference") (OtherBodyIndex :type Integer) (bFromSweep :type Boolean) (SweepResult :type "HitResult Structure (by ref)"))
  ;[1 1 1] Set Location Type
  (`self.CheckJari` OtherActor OtherComp
    (:`Out`
      (set `self.XYZ` 1))))

(event `self.ReceiveBeginPlay`)

(event `self.StaticMesh18.OnComponentBeginOverlap`
  (params (OverlappedComponent :type "PrimitiveComponent Object Reference") (OtherActor :type "Actor Object Reference") (OtherComp :type "PrimitiveComponent Object Reference") (OtherBodyIndex :type Integer) (bFromSweep :type Boolean) (SweepResult :type "HitResult Structure (by ref)"))
  ;[1 1 1] Set Location
  (`self.CheckJari` OtherActor OtherComp
    (:`Out`
      (`self.Location` -20.0 (`self.XYZ`)))))

(event `self.StaticMesh5.OnComponentBeginOverlap`
  (params (OverlappedComponent :type "PrimitiveComponent Object Reference") (OtherActor :type "Actor Object Reference") (OtherComp :type "PrimitiveComponent Object Reference") (OtherBodyIndex :type Integer) (bFromSweep :type Boolean) (SweepResult :type "HitResult Structure (by ref)"))
  ;[1 1 1] Set Location Type
  (`self.CheckJari` OtherActor OtherComp
    (:`Out`
      (set `self.XYZ` 2))))

(event `self.StaticMesh2.OnComponentBeginOverlap`
  (params (OverlappedComponent :type "PrimitiveComponent Object Reference") (OtherActor :type "Actor Object Reference") (OtherComp :type "PrimitiveComponent Object Reference") (OtherBodyIndex :type Integer) (bFromSweep :type Boolean) (SweepResult :type "HitResult Structure (by ref)"))
  ;[1 1 1] Set Color Type
  (`self.CheckJari` OtherActor OtherComp
    (:`Out`
      (set `self.RGB` 0))))

(event `self.StaticMesh4.OnComponentBeginOverlap`
  (params (OverlappedComponent :type "PrimitiveComponent Object Reference") (OtherActor :type "Actor Object Reference") (OtherComp :type "PrimitiveComponent Object Reference") (OtherBodyIndex :type Integer) (bFromSweep :type Boolean) (SweepResult :type "HitResult Structure (by ref)"))
  ;[1 1 1] SetColor
  (`self.CheckJari` OtherActor OtherComp
    (:`Out`
      (`self.Color` 0.1 (`self.RGB`)))))

(event `self.StaticMesh8.OnComponentBeginOverlap`
  (params (OverlappedComponent :type "PrimitiveComponent Object Reference") (OtherActor :type "Actor Object Reference") (OtherComp :type "PrimitiveComponent Object Reference") (OtherBodyIndex :type Integer) (bFromSweep :type Boolean) (SweepResult :type "HitResult Structure (by ref)"))
  (bind _pointlight (`/Game/Bulb/BP_Lampu.PointLight` (`|GetArrayItem` (`self.AllLamp`) (`self.OnIndex`))))
  ;[1 1 1] Inetnsity
  (`self.CheckJari` OtherActor OtherComp
    (:`Out`
      (`LightComponent.SetIntensity` _pointlight (+ 1000.0 (`LightComponentBase.Intensity` _pointlight))))))

(event `self.StaticMesh1.OnComponentBeginOverlap`
  (params (OverlappedComponent :type "PrimitiveComponent Object Reference") (OtherActor :type "Actor Object Reference") (OtherComp :type "PrimitiveComponent Object Reference") (OtherBodyIndex :type Integer) (bFromSweep :type Boolean) (SweepResult :type "HitResult Structure (by ref)"))
  ;[1 1 1] Set Color Type
  (`self.CheckJari` OtherActor OtherComp
    (:`Out`
      (set `self.RGB` 1))))

(event `self.StaticMesh3.OnComponentBeginOverlap`
  (params (OverlappedComponent :type "PrimitiveComponent Object Reference") (OtherActor :type "Actor Object Reference") (OtherComp :type "PrimitiveComponent Object Reference") (OtherBodyIndex :type Integer) (bFromSweep :type Boolean) (SweepResult :type "HitResult Structure (by ref)"))
  ;[1 1 1] SetColor
  (`self.CheckJari` OtherActor OtherComp
    (:`Out`
      (`self.Color` -0.1 (`self.RGB`)))))

(event `self.StaticMesh9.OnComponentBeginOverlap`
  (params (OverlappedComponent :type "PrimitiveComponent Object Reference") (OtherActor :type "Actor Object Reference") (OtherComp :type "PrimitiveComponent Object Reference") (OtherBodyIndex :type Integer) (bFromSweep :type Boolean) (SweepResult :type "HitResult Structure (by ref)"))
  (bind _pointlight (`/Game/Bulb/BP_Lampu.PointLight` (`|GetArrayItem` (`self.AllLamp`) (`self.OnIndex`))))
  ;[1 1 1] Inetnsity
  (`self.CheckJari` OtherActor OtherComp
    (:`Out`
      (`LightComponent.SetIntensity` _pointlight (+ -1000.0 (`LightComponentBase.Intensity` _pointlight))))))

(event `self.StaticMesh.OnComponentBeginOverlap`
  (params (OverlappedComponent :type "PrimitiveComponent Object Reference") (OtherActor :type "Actor Object Reference") (OtherComp :type "PrimitiveComponent Object Reference") (OtherBodyIndex :type Integer) (bFromSweep :type Boolean) (SweepResult :type "HitResult Structure (by ref)"))
  ;[1 1 1] Set Color Type
  (`self.CheckJari` OtherActor OtherComp
    (:`Out`
      (set `self.RGB` 2))))

(event `self.StaticMesh14.OnComponentBeginOverlap`
  (params (OverlappedComponent :type "PrimitiveComponent Object Reference") (OtherActor :type "Actor Object Reference") (OtherComp :type "PrimitiveComponent Object Reference") (OtherBodyIndex :type Integer) (bFromSweep :type Boolean) (SweepResult :type "HitResult Structure (by ref)"))
  (bind _alllamp (`self.AllLamp`))
  (bind _returnvalue (`KismetArrayLibrary.Array_LastIndex` _alllamp))
  (bind _returnvalue_2 (- (`self.OnIndex`) 1))
  ;[1 1 1] RemoveLamp
  (`self.CheckJari` OtherActor OtherComp
    (:`Out`
      (if (<= (`self.OnIndex`) _returnvalue)
        (`self.K2_DestroyActor` (`|GetArrayItem` (`self.AllLamp`) (`self.OnIndex`)))
        (`KismetArrayLibrary.Array_Remove` (`self.AllLamp`) (`self.OnIndex`))
        (if (and (== _returnvalue_2 _returnvalue) (not (== (`KismetArrayLibrary.Array_Length` _alllamp) 0)))
          (bind _output_get (set `self.OnIndex` _returnvalue_2)))
        (`SceneComponent.K2_SetWorldLocation` (`self.PickLampu`) (`SceneComponent.K2_GetComponentLocation` (`/Game/Bulb/BP_Lampu.DefaultSceneRoot` (`|GetArrayItem` (`self.AllLamp`) (`self.OnIndex`)))) false false)
        (`TextRenderComponent.K2_SetText` (`self.TextRender2`) (`KismetTextLibrary.Conv_IntToText` _output_get))))))

(event `self.StaticMesh13.OnComponentBeginOverlap`
  (params (OverlappedComponent :type "PrimitiveComponent Object Reference") (OtherActor :type "Actor Object Reference") (OtherComp :type "PrimitiveComponent Object Reference") (OtherBodyIndex :type Integer) (bFromSweep :type Boolean) (SweepResult :type "HitResult Structure (by ref)"))
  ;[1 1 1] SpawnLamp
  (`self.CheckJari` OtherActor OtherComp
    (:`Out`
      (bind _returnvalue (`|SpawnActorFromClass` "/Game/Bulb/BP_Lampu.BP_Lampu_C" (`KismetMathLibrary.MakeTransform` (`SceneComponent.K2_GetComponentLocation` (`self.SpawnPoint`))) "Undefined" "MultiplyWithRoot" null null))
      (bind _returnvalue_2 (`KismetArrayLibrary.Array_Add` (`self.AllLamp`) _returnvalue))
      (bind _output_get (set `self.OnIndex` _returnvalue_2))
      (`SceneComponent.K2_SetWorldLocation` (`self.PickLampu`) (`SceneComponent.K2_GetComponentLocation` (`self.SpawnPoint`)) false false)
      (`TextRenderComponent.K2_SetText` (`self.TextRender2`) (`KismetTextLibrary.Conv_IntToText` _output_get)))))

(event `self.StaticMesh10.OnComponentBeginOverlap`
  (params (OverlappedComponent :type "PrimitiveComponent Object Reference") (OtherActor :type "Actor Object Reference") (OtherComp :type "PrimitiveComponent Object Reference") (OtherBodyIndex :type Integer) (bFromSweep :type Boolean) (SweepResult :type "HitResult Structure (by ref)"))
  ;[1 1 1] PickingIndex
  (`self.CheckJari` OtherActor OtherComp
    (:`Out`
      (if (< (`self.OnIndex`) (`KismetArrayLibrary.Array_LastIndex` (`self.AllLamp`)))
        (bind _output_get (set `self.OnIndex` (+ (`self.OnIndex`) 1)))
        (`SceneComponent.K2_SetWorldLocation` (`self.PickLampu`) (`SceneComponent.K2_GetComponentLocation` (`/Game/Bulb/BP_Lampu.DefaultSceneRoot` (`|GetArrayItem` (`self.AllLamp`) (`self.OnIndex`)))) false false)
        (`TextRenderComponent.K2_SetText` (`self.TextRender2`) (`KismetTextLibrary.Conv_IntToText` _output_get))))))

(event `self.StaticMesh12.OnComponentBeginOverlap`
  (params (OverlappedComponent :type "PrimitiveComponent Object Reference") (OtherActor :type "Actor Object Reference") (OtherComp :type "PrimitiveComponent Object Reference") (OtherBodyIndex :type Integer) (bFromSweep :type Boolean) (SweepResult :type "HitResult Structure (by ref)"))
  ;[1 1 1] PickingIndex
  (`self.CheckJari` OtherActor OtherComp
    (:`Out`
      (if (> (`self.OnIndex`) 0)
        (bind _output_get (set `self.OnIndex` (+ (`self.OnIndex`) -1)))
        (`SceneComponent.K2_SetWorldLocation` (`self.PickLampu`) (`SceneComponent.K2_GetComponentLocation` (`/Game/Bulb/BP_Lampu.DefaultSceneRoot` (`|GetArrayItem` (`self.AllLamp`) (`self.OnIndex`)))) false false)
        (`TextRenderComponent.K2_SetText` (`self.TextRender2`) (`KismetTextLibrary.Conv_IntToText` _output_get))))))

(fn `UserConstructionScript`)