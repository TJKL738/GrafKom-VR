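; VR control table that drives a BP_Camer child actor through buttons touched by the player's index fingers.
; CheckJari filters every button overlap to the VRPawnManual's left or right index finger component.
; Five cubes select a camera index, three meshes choose the X/Y/Z axis, and another triggers PlayAnimation.
; Step buttons nudge the selected Location or Rotator array entry along that axis, then call the camera's Move or Rot.
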(event `self.ReceiveBeginPlay`
  (bind _asbp_camer (cast `/Game/VR_Things/Blueprint/CameraLighting/BP_Camer` (`ChildActorComponent.ChildActor` (`self.BP_Camer`))))
  (set `self.As BP Camer` _asbp_camer))

(event `self.Cube.OnComponentBeginOverlap`
  (params (OverlappedComponent :type "PrimitiveComponent Object Reference") (OtherActor :type "Actor Object Reference") (OtherComp :type "PrimitiveComponent Object Reference") (OtherBodyIndex :type Integer) (bFromSweep :type Boolean) (SweepResult :type "HitResult Structure (by ref)"))
  (bind _as_bp_camer (`self.As BP Camer`))
  (`self.CheckJari` OtherActor OtherComp
    (:`Out`
      (set `/Game/VR_Things/Blueprint/CameraLighting/BP_Camer.Index` 0 _as_bp_camer)
      (`/Game/VR_Things/Blueprint/CameraLighting/BP_Camer.Move` _as_bp_camer)
      (`/Game/VR_Things/Blueprint/CameraLighting/BP_Camer.Rot` _as_bp_camer))))

(event `self.Cube1.OnComponentBeginOverlap`
  (params (OverlappedComponent :type "PrimitiveComponent Object Reference") (OtherActor :type "Actor Object Reference") (OtherComp :type "PrimitiveComponent Object Reference") (OtherBodyIndex :type Integer) (bFromSweep :type Boolean) (SweepResult :type "HitResult Structure (by ref)"))
  (bind _as_bp_camer (`self.As BP Camer`))
  (`self.CheckJari` OtherActor OtherComp
    (:`Out`
      (set `/Game/VR_Things/Blueprint/CameraLighting/BP_Camer.Index` 1 _as_bp_camer)
      (`/Game/VR_Things/Blueprint/CameraLighting/BP_Camer.Move` _as_bp_camer)
      (`/Game/VR_Things/Blueprint/CameraLighting/BP_Camer.Rot` _as_bp_camer))))

(event `self.Cube2.OnComponentBeginOverlap`
  (params (OverlappedComponent :type "PrimitiveComponent Object Reference") (OtherActor :type "Actor Object Reference") (OtherComp :type "PrimitiveComponent Object Reference") (OtherBodyIndex :type Integer) (bFromSweep :type Boolean) (SweepResult :type "HitResult Structure (by ref)"))
  (bind _as_bp_camer (`self.As BP Camer`))
  (`self.CheckJari` OtherActor OtherComp
    (:`Out`
      (set `/Game/VR_Things/Blueprint/CameraLighting/BP_Camer.Index` 2 _as_bp_camer)
      (`/Game/VR_Things/Blueprint/CameraLighting/BP_Camer.Move` _as_bp_camer)
      (`/Game/VR_Things/Blueprint/CameraLighting/BP_Camer.Rot` _as_bp_camer))))

(event `self.Cube3.OnComponentBeginOverlap`
  (params (OverlappedComponent :type "PrimitiveComponent Object Reference") (OtherActor :type "Actor Object Reference") (OtherComp :type "PrimitiveComponent Object Reference") (OtherBodyIndex :type Integer) (bFromSweep :type Boolean) (SweepResult :type "HitResult Structure (by ref)"))
  (bind _as_bp_camer (`self.As BP Camer`))
  (`self.CheckJari` OtherActor OtherComp
    (:`Out`
      (set `/Game/VR_Things/Blueprint/CameraLighting/BP_Camer.Index` 3 _as_bp_camer)
      (`/Game/VR_Things/Blueprint/CameraLighting/BP_Camer.Move` _as_bp_camer)
      (`/Game/VR_Things/Blueprint/CameraLighting/BP_Camer.Rot` _as_bp_camer))))

(event `self.Cube4.OnComponentBeginOverlap`
  (params (OverlappedComponent :type "PrimitiveComponent Object Reference") (OtherActor :type "Actor Object Reference") (OtherComp :type "PrimitiveComponent Object Reference") (OtherBodyIndex :type Integer) (bFromSweep :type Boolean) (SweepResult :type "HitResult Structure (by ref)"))
  (bind _as_bp_camer (`self.As BP Camer`))
  (`self.CheckJari` OtherActor OtherComp
    (:`Out`
      (set `/Game/VR_Things/Blueprint/CameraLighting/BP_Camer.Index` 4 _as_bp_camer)
      (`/Game/VR_Things/Blueprint/CameraLighting/BP_Camer.Move` _as_bp_camer)
      (`/Game/VR_Things/Blueprint/CameraLighting/BP_Camer.Rot` _as_bp_camer))))

(event `self.StaticMesh2.OnComponentBeginOverlap`
  (params (OverlappedComponent :type "PrimitiveComponent Object Reference") (OtherActor :type "Actor Object Reference") (OtherComp :type "PrimitiveComponent Object Reference") (OtherBodyIndex :type Integer) (bFromSweep :type Boolean) (SweepResult :type "HitResult Structure (by ref)"))
  (`self.CheckJari` OtherActor OtherComp
    (:`Out`
      (set `self.XYZ` 0))))

(event `self.StaticMesh1.OnComponentBeginOverlap`
  (params (OverlappedComponent :type "PrimitiveComponent Object Reference") (OtherActor :type "Actor Object Reference") (OtherComp :type "PrimitiveComponent Object Reference") (OtherBodyIndex :type Integer) (bFromSweep :type Boolean) (SweepResult :type "HitResult Structure (by ref)"))
  (`self.CheckJari` OtherActor OtherComp
    (:`Out`
      (set `self.XYZ` 1))))

(event `self.StaticMesh.OnComponentBeginOverlap`
  (params (OverlappedComponent :type "PrimitiveComponent Object Reference") (OtherActor :type "Actor Object Reference") (OtherComp :type "PrimitiveComponent Object Reference") (OtherBodyIndex :type Integer) (bFromSweep :type Boolean) (SweepResult :type "HitResult Structure (by ref)"))
  (`self.CheckJari` OtherActor OtherComp
    (:`Out`
      (set `self.XYZ` 2))))

(event `self.StaticMesh3.OnComponentBeginOverlap`
  (params (OverlappedComponent :type "PrimitiveComponent Object Reference") (OtherActor :type "Actor Object Reference") (OtherComp :type "PrimitiveComponent Object Reference") (OtherBodyIndex :type Integer) (bFromSweep :type Boolean) (SweepResult :type "HitResult Structure (by ref)"))
  (`self.CheckJari` OtherActor OtherComp
    (:`Out`
      (`self.LocationSetting` -20.0
        (:`Out`
          (`/Game/VR_Things/Blueprint/CameraLighting/BP_Camer.Move` (`self.As BP Camer`)))))))

(event `self.StaticMesh4.OnComponentBeginOverlap`
  (params (OverlappedComponent :type "PrimitiveComponent Object Reference") (OtherActor :type "Actor Object Reference") (OtherComp :type "PrimitiveComponent Object Reference") (OtherBodyIndex :type Integer) (bFromSweep :type Boolean) (SweepResult :type "HitResult Structure (by ref)"))
  (`self.CheckJari` OtherActor OtherComp
    (:`Out`
      (`self.LocationSetting` 20.0
        (:`Out`
          (`/Game/VR_Things/Blueprint/CameraLighting/BP_Camer.Move` (`self.As BP Camer`)))))))

(event `PlayAnimation`
  (`/Game/VR_Things/Blueprint/CameraLighting/BP_Camer.PlayAnimation` (`self.As BP Camer`) :!label _label))

(event `self.StaticMesh5.OnComponentBeginOverlap`
  (params (OverlappedComponent :type "PrimitiveComponent Object Reference") (OtherActor :type "Actor Object Reference") (OtherComp :type "PrimitiveComponent Object Reference") (OtherBodyIndex :type Integer) (bFromSweep :type Boolean) (SweepResult :type "HitResult Structure (by ref)"))
  (`self.CheckJari` OtherActor OtherComp
    (:`Out`
      (goto _label))))

(event `self.StaticMesh9.OnComponentBeginOverlap`
  (params (OverlappedComponent :type "PrimitiveComponent Object Reference") (OtherActor :type "Actor Object Reference") (OtherComp :type "PrimitiveComponent Object Reference") (OtherBodyIndex :type Integer) (bFromSweep :type Boolean) (SweepResult :type "HitResult Structure (by ref)"))
  (`self.CheckJari` OtherActor OtherComp
    (:`Out`
      (`self.RotationSetting` -10.0
        (:`Out`
          (`/Game/VR_Things/Blueprint/CameraLighting/BP_Camer.Rot` (`self.As BP Camer`)))))))

(event `self.StaticMesh8.OnComponentBeginOverlap`
  (params (OverlappedComponent :type "PrimitiveComponent Object Reference") (OtherActor :type "Actor Object Reference") (OtherComp :type "PrimitiveComponent Object Reference") (OtherBodyIndex :type Integer) (bFromSweep :type Boolean) (SweepResult :type "HitResult Structure (by ref)"))
  (`self.CheckJari` OtherActor OtherComp
    (:`Out`
      (`self.RotationSetting` 10.0
        (:`Out`
          (`/Game/VR_Things/Blueprint/CameraLighting/BP_Camer.Rot` (`self.As BP Camer`)))))))

(fn `UserConstructionScript`)