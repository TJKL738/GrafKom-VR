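; VR table Blueprint that spawns a 3D shape, such as a cube or hyperboloid, when a pawn's index finger touches its collision trigger.
; SpawnObject replaces the previous shape at SpawnTable and broadcasts EDObjectIsSpawned.
; BLEDOSIN then blasts the trigger's paired geometry collection with a radial impulse if the pawn's LAGIMARAH flag is set.
; SpawnObjectWithoutChecking offers the same spawn without the finger check or blast.
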(event `self.SphereCol.OnComponentBeginOverlap`
  (params (OverlappedComponent :type "PrimitiveComponent Object Reference") (OtherActor :type "Actor Object Reference") (OtherComp :type "PrimitiveComponent Object Reference") (OtherBodyIndex :type Integer) (bFromSweep :type Boolean) (SweepResult :type "HitResult Structure (by ref)"))
  ;[1 1 1] Spawn Object
  (`self.SpawnObject` OtherActor "/Game/OBJECT/Sphere.Sphere_C" OtherComp (`self.Cube_GeometryCollection5`)))

(event `self.ReceiveBeginPlay`)

(event `self.CubeCol.OnComponentBeginOverlap`
  (params (OverlappedComponent :type "PrimitiveComponent Object Reference") (OtherActor :type "Actor Object Reference") (OtherComp :type "PrimitiveComponent Object Reference") (OtherBodyIndex :type Integer) (bFromSweep :type Boolean) (SweepResult :type "HitResult Structure (by ref)"))
  ;[1 1 1] Spawn Object
  (`self.SpawnObject` OtherActor "/Game/OBJECT/Cube.Cube_C" OtherComp (`self.Cube_GeometryCollection1`)))

(event `self.HyperboloidCol.OnComponentBeginOverlap`
  (params (OverlappedComponent :type "PrimitiveComponent Object Reference") (OtherActor :type "Actor Object Reference") (OtherComp :type "PrimitiveComponent Object Reference") (OtherBodyIndex :type Integer) (bFromSweep :type Boolean) (SweepResult :type "HitResult Structure (by ref)"))
  ;[1 1 1] Spawn Object
  (`self.SpawnObject` OtherActor "/Game/OBJECT/Hyperboloid.Hyperboloid_C" OtherComp (`self.Cube_GeometryCollection4`)))

(event `self.CylinderCol.OnComponentBeginOverlap`
  (params (OverlappedComponent :type "PrimitiveComponent Object Reference") (OtherActor :type "Actor Object Reference") (OtherComp :type "PrimitiveComponent Object Reference") (OtherBodyIndex :type Integer) (bFromSweep :type Boolean) (SweepResult :type "HitResult Structure (by ref)"))
  ;[1 1 1] Spawn Object
  (`self.SpawnObject` OtherActor "/Game/OBJECT/Cylinder.Cylinder_C" OtherComp (`self.Cube_GeometryCollection3`)))

(event `self.hyperbolic paraboloid Col.OnComponentBeginOverlap`
  (params (OverlappedComponent :type "PrimitiveComponent Object Reference") (OtherActor :type "Actor Object Reference") (OtherComp :type "PrimitiveComponent Object Reference") (OtherBodyIndex :type Integer) (bFromSweep :type Boolean) (SweepResult :type "HitResult Structure (by ref)"))
  ;[1 1 1] Spawn Object
  (`self.SpawnObject` OtherActor "/Game/OBJECT/HyperbolIcParaboloid.HyperbolIcParaboloid_C" OtherComp (`self.Cube_GeometryCollection`)))

(event `self.elliptic paraboloid Col.OnComponentBeginOverlap`
  (params (OverlappedComponent :type "PrimitiveComponent Object Reference") (OtherActor :type "Actor Object Reference") (OtherComp :type "PrimitiveComponent Object Reference") (OtherBodyIndex :type Integer) (bFromSweep :type Boolean) (SweepResult :type "HitResult Structure (by ref)"))
  ;[1 1 1] Spawn Object
  (`self.SpawnObject` OtherActor "/Game/OBJECT/ElipticParaboloid.ElipticParaboloid_C" OtherComp (`self.Cube_GeometryCollection2`)))

(fn `UserConstructionScript`)