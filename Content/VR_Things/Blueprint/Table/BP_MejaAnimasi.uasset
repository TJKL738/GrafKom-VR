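; VR animation table whose touch buttons, pressed by either index finger of VRPawnManual, pose and play animation on BP_SkelRob.
; Five cubes set the skeleton's Index and refresh its Animation, while three meshes choose the roll, pitch or yaw axis.
; Two meshes nudge that axis of the indexed Seq.Rot entry up or down through Rot, and another calls PlayA.
; SpawnObject, which replaces a spawned actor, is never called here.
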(event `self.ReceiveBeginPlay`
  (bind _returnvalue (`GameplayStatics.GetActorOfClass` "/Game/VR_Things/Blueprint/Object/BP_Robot.BP_Robot_C"))
  (set `self.Robot` _returnvalue)
  (bind _returnvalue_2 (`GameplayStatics.GetActorOfClass` "/Game/VR_Things/Blueprint/Skeleton/BP_SkelRob.BP_SkelRob_C"))
  (set `self.Skel` _returnvalue_2))

(event `self.Cube.OnComponentBeginOverlap`
  (params (OverlappedComponent :type "PrimitiveComponent Object Reference") (OtherActor :type "Actor Object Reference") (OtherComp :type "PrimitiveComponent Object Reference") (OtherBodyIndex :type Integer) (bFromSweep :type Boolean) (SweepResult :type "HitResult Structure (by ref)"))
  (bind _asvrpawn_manual (cast `/Game/VR_Things/Blueprint/BP_GameThings/VRPawnManual` OtherActor))
  (if (or (== (`/Game/VR_Things/Blueprint/BP_GameThings/VRPawnManual.IndexLeft` _asvrpawn_manual) OtherComp) (== (`/Game/VR_Things/Blueprint/BP_GameThings/VRPawnManual.IndexRight` _asvrpawn_manual) OtherComp))
    (bind _returnvalue (`GameplayStatics.GetActorOfClass` "/Game/VR_Things/Blueprint/Skeleton/BP_SkelRob.BP_SkelRob_C"))
    (set `/Game/VR_Things/Blueprint/Skeleton/BP_SkelRob.Index` 0 _returnvalue)
    (`/Game/VR_Things/Blueprint/Skeleton/BP_SkelRob.Animation` _returnvalue)))

(event `self.Cube1.OnComponentBeginOverlap`
  (params (OverlappedComponent :type "PrimitiveComponent Object Reference") (OtherActor :type "Actor Object Reference") (OtherComp :type "PrimitiveComponent Object Reference") (OtherBodyIndex :type Integer) (bFromSweep :type Boolean) (SweepResult :type "HitResult Structure (by ref)"))
  (bind _asvrpawn_manual (cast `/Game/VR_Things/Blueprint/BP_GameThings/VRPawnManual` OtherActor))
  (if (or (== (`/Game/VR_Things/Blueprint/BP_GameThings/VRPawnManual.IndexLeft` _asvrpawn_manual) OtherComp) (== (`/Game/VR_Things/Blueprint/BP_GameThings/VRPawnManual.IndexRight` _asvrpawn_manual) OtherComp))
    (bind _returnvalue (`GameplayStatics.GetActorOfClass` "/Game/VR_Things/Blueprint/Skeleton/BP_SkelRob.BP_SkelRob_C"))
    (set `/Game/VR_Things/Blueprint/Skeleton/BP_SkelRob.Index` 1 _returnvalue)
    (`/Game/VR_Things/Blueprint/Skeleton/BP_SkelRob.Animation` _returnvalue)))

(event `self.Cube2.OnComponentBeginOverlap`
  (params (OverlappedComponent :type "PrimitiveComponent Object Reference") (OtherActor :type "Actor Object Reference") (OtherComp :type "PrimitiveComponent Object Reference") (OtherBodyIndex :type Integer) (bFromSweep :type Boolean) (SweepResult :type "HitResult Structure (by ref)"))
  (bind _asvrpawn_manual (cast `/Game/VR_Things/Blueprint/BP_GameThings/VRPawnManual` OtherActor))
  (if (or (== (`/Game/VR_Things/Blueprint/BP_GameThings/VRPawnManual.IndexLeft` _asvrpawn_manual) OtherComp) (== (`/Game/VR_Things/Blueprint/BP_GameThings/VRPawnManual.IndexRight` _asvrpawn_manual) OtherComp))
    (bind _returnvalue (`GameplayStatics.GetActorOfClass` "/Game/VR_Things/Blueprint/Skeleton/BP_SkelRob.BP_SkelRob_C"))
    (set `/Game/VR_Things/Blueprint/Skeleton/BP_SkelRob.Index` 2 _returnvalue)
    (`/Game/VR_Things/Blueprint/Skeleton/BP_SkelRob.Animation` _returnvalue)))

(event `self.Cube3.OnComponentBeginOverlap`
  (params (OverlappedComponent :type "PrimitiveComponent Object Reference") (OtherActor :type "Actor Object Reference") (OtherComp :type "PrimitiveComponent Object Reference") (OtherBodyIndex :type Integer) (bFromSweep :type Boolean) (SweepResult :type "HitResult Structure (by ref)"))
  (bind _asvrpawn_manual (cast `/Game/VR_Things/Blueprint/BP_GameThings/VRPawnManual` OtherActor))
  (if (or (== (`/Game/VR_Things/Blueprint/BP_GameThings/VRPawnManual.IndexLeft` _asvrpawn_manual) OtherComp) (== (`/Game/VR_Things/Blueprint/BP_GameThings/VRPawnManual.IndexRight` _asvrpawn_manual) OtherComp))
    (bind _returnvalue (`GameplayStatics.GetActorOfClass` "/Game/VR_Things/Blueprint/Skeleton/BP_SkelRob.BP_SkelRob_C"))
    (set `/Game/VR_Things/Blueprint/Skeleton/BP_SkelRob.Index` 3 _returnvalue)
    (`/Game/VR_Things/Blueprint/Skeleton/BP_SkelRob.Animation` _returnvalue)))

(event `self.Cube4.OnComponentBeginOverlap`
  (params (OverlappedComponent :type "PrimitiveComponent Object Reference") (OtherActor :type "Actor Object Reference") (OtherComp :type "PrimitiveComponent Object Reference") (OtherBodyIndex :type Integer) (bFromSweep :type Boolean) (SweepResult :type "HitResult Structure (by ref)"))
  (bind _asvrpawn_manual (cast `/Game/VR_Things/Blueprint/BP_GameThings/VRPawnManual` OtherActor))
  (if (or (== (`/Game/VR_Things/Blueprint/BP_GameThings/VRPawnManual.IndexLeft` _asvrpawn_manual) OtherComp) (== (`/Game/VR_Things/Blueprint/BP_GameThings/VRPawnManual.IndexRight` _asvrpawn_manual) OtherComp))
    (bind _returnvalue (`GameplayStatics.GetActorOfClass` "/Game/VR_Things/Blueprint/Skeleton/BP_SkelRob.BP_SkelRob_C"))
    (set `/Game/VR_Things/Blueprint/Skeleton/BP_SkelRob.Index` 4 _returnvalue)
    (`/Game/VR_Things/Blueprint/Skeleton/BP_SkelRob.Animation` _returnvalue)))

(event `self.StaticMesh2.OnComponentBeginOverlap`
  (params (OverlappedComponent :type "PrimitiveComponent Object Reference") (OtherActor :type "Actor Object Reference") (OtherComp :type "PrimitiveComponent Object Reference") (OtherBodyIndex :type Integer) (bFromSweep :type Boolean) (SweepResult :type "HitResult Structure (by ref)"))
  (bind _asvrpawn_manual (cast `/Game/VR_Things/Blueprint/BP_GameThings/VRPawnManual` OtherActor))
  (if (or (== (`/Game/VR_Things/Blueprint/BP_GameThings/VRPawnManual.IndexLeft` _asvrpawn_manual) OtherComp) (== (`/Game/VR_Things/Blueprint/BP_GameThings/VRPawnManual.IndexRight` _asvrpawn_manual) OtherComp))
    (set `self.XYZ` 0)))

(event `self.StaticMesh1.OnComponentBeginOverlap`
  (params (OverlappedComponent :type "PrimitiveComponent Object Reference") (OtherActor :type "Actor Object Reference") (OtherComp :type "PrimitiveComponent Object Reference") (OtherBodyIndex :type Integer) (bFromSweep :type Boolean) (SweepResult :type "HitResult Structure (by ref)"))
  (bind _asvrpawn_manual (cast `/Game/VR_Things/Blueprint/BP_GameThings/VRPawnManual` OtherActor))
  (if (or (== (`/Game/VR_Things/Blueprint/BP_GameThings/VRPawnManual.IndexLeft` _asvrpawn_manual) OtherComp) (== (`/Game/VR_Things/Blueprint/BP_GameThings/VRPawnManual.IndexRight` _asvrpawn_manual) OtherComp))
    (set `self.XYZ` 1)))

(event `self.StaticMesh.OnComponentBeginOverlap`
  (params (OverlappedComponent :type "PrimitiveComponent Object Reference") (OtherActor :type "Actor Object Reference") (OtherComp :type "PrimitiveComponent Object Reference") (OtherBodyIndex :type Integer) (bFromSweep :type Boolean) (SweepResult :type "HitResult Structure (by ref)"))
  (bind _asvrpawn_manual (cast `/Game/VR_Things/Blueprint/BP_GameThings/VRPawnManual` OtherActor))
  (if (or (== (`/Game/VR_Things/Blueprint/BP_GameThings/VRPawnManual.IndexLeft` _asvrpawn_manual) OtherComp) (== (`/Game/VR_Things/Blueprint/BP_GameThings/VRPawnManual.IndexRight` _asvrpawn_manual) OtherComp))
    (set `self.XYZ` 2)))

(event `self.StaticMesh3.OnComponentBeginOverlap`
  (params (OverlappedComponent :type "PrimitiveComponent Object Reference") (OtherActor :type "Actor Object Reference") (OtherComp :type "PrimitiveComponent Object Reference") (OtherBodyIndex :type Integer) (bFromSweep :type Boolean) (SweepResult :type "HitResult Structure (by ref)"))
  (bind _asvrpawn_manual (cast `/Game/VR_Things/Blueprint/BP_GameThings/VRPawnManual` OtherActor))
  (if (or (== (`/Game/VR_Things/Blueprint/BP_GameThings/VRPawnManual.IndexLeft` _asvrpawn_manual) OtherComp) (== (`/Game/VR_Things/Blueprint/BP_GameThings/VRPawnManual.IndexRight` _asvrpawn_manual) OtherComp))
    (`self.Rot` -20.0
      (:`Out`
        (`/Game/VR_Things/Blueprint/Skeleton/BP_SkelRob.Animation` (`self.Skel`))))))

(event `self.StaticMesh4.OnComponentBeginOverlap`
  (params (OverlappedComponent :type "PrimitiveComponent Object Reference") (OtherActor :type "Actor Object Reference") (OtherComp :type "PrimitiveComponent Object Reference") (OtherBodyIndex :type Integer) (bFromSweep :type Boolean) (SweepResult :type "HitResult Structure (by ref)"))
  (bind _asvrpawn_manual (cast `/Game/VR_Things/Blueprint/BP_GameThings/VRPawnManual` OtherActor))
  (if (or (== (`/Game/VR_Things/Blueprint/BP_GameThings/VRPawnManual.IndexLeft` _asvrpawn_manual) OtherComp) (== (`/Game/VR_Things/Blueprint/BP_GameThings/VRPawnManual.IndexRight` _asvrpawn_manual) OtherComp))
    (`self.Rot` 20.0
      (:`Out`
        (`/Game/VR_Things/Blueprint/Skeleton/BP_SkelRob.Animation` (`self.Skel`))))))

(event `self.StaticMesh5.OnComponentBeginOverlap`
  (params (OverlappedComponent :type "PrimitiveComponent Object Reference") (OtherActor :type "Actor Object Reference") (OtherComp :type "PrimitiveComponent Object Reference") (OtherBodyIndex :type Integer) (bFromSweep :type Boolean) (SweepResult :type "HitResult Structure (by ref)"))
  (bind _asvrpawn_manual (cast `/Game/VR_Things/Blueprint/BP_GameThings/VRPawnManual` OtherActor))
  (if (or (== (`/Game/VR_Things/Blueprint/BP_GameThings/VRPawnManual.IndexLeft` _asvrpawn_manual) OtherComp) (== (`/Game/VR_Things/Blueprint/BP_GameThings/VRPawnManual.IndexRight` _asvrpawn_manual) OtherComp))
    (`/Game/VR_Things/Blueprint/Skeleton/BP_SkelRob.PlayA` (`self.Skel`))))

(fn `UserConstructionScript`)