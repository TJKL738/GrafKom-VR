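; BP_RobotPlayable is a robot object for the VR project, built from separate body-part components with Indonesian names (head, body, shoulders, elbows, hands, thighs, knees, feet).
; On BeginPlay, Start sets the visibility of every model component from the IsModel flag without propagating to children.
; It then fills MainRoot with the fourteen named body parts.
; NewMacro holds an unreachable copy of this logic with a debug print.
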(event `self.ReceiveBeginPlay`
  (`self.Start`)
  (`parent.ReceiveBeginPlay`))

(fn `Start`
  (bind _output_get (set `self.ModelComponent` (`|MakeArray` (`self.KakiKiri`) (`self.KakiKanan`) (`self.3`) (`self.4`) (`self.LututKiri`) (`self.LututKanan`) (`self.7`) (`self.8`) (`self.PahaKiri`) (`self.PahaKanan`) (`self.Badan`) (`self.12`) (`self.13`) (`self.14`) (`self.15`) (`self.16`) (`self.17`) (`self.PundakKiri`) (`self.19`) (`self.SikuKiri`) (`self.21`) (`self.TanganKiri`) (`self.PundakKanan`) (`self.24`) (`self.SikuKanan`) (`self.26`) (`self.TanganKanan`) (`self.28`) (`self.Kepala`) (`self.30`) (`self.31`) (`self.32`) (`self.33`) (`self.34`))))
  (for _array_element _output_get
    (`SceneComponent.SetVisibility` _array_element (`self.isModel?`) false))
  (set `self.MainRoot` (`|MakeArray` (`self.Badan`) (`self.Kepala`) (`self.PundakKiri`) (`self.PundakKanan`) (`self.SikuKiri`) (`self.SikuKanan`) (`self.TanganKiri`) (`self.TanganKanan`) (`self.PahaKiri`) (`self.PahaKanan`) (`self.LututKiri`) (`self.LututKanan`) (`self.KakiKiri`) (`self.KakiKanan`)))
  (return))

(fn `UserConstructionScript`
  (`parent.UserConstructionScript`))