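; VR robot actor built from jointed body-part components with Indonesian names, playing a looping example animation from BeginPlay.
; Start sets every model part's visibility from IsModel and fills the MainRoot array with the main joints.
; RobotAnimationExample alternates two timelines that swing shoulders, elbows, head and thighs between two poses.
; Each update lerps from the joint's current relative rotation, so motion compounds rather than following the curve directly.
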(event `self.ReceiveBeginPlay`
  (`self.Start`)
  (`parent.ReceiveBeginPlay`)
  (`self.Robot Animation Example`))

(event `Robot Animation Example`
  (bind _pundakkanan (`self.PundakKanan`))
  (bind _pundakkanan_2 (`self.PundakKanan`))
  (bind _sikukanan (`self.SikuKanan`))
  (bind _pundakkiri (`self.PundakKiri`))
  (bind _sikukiri (`self.SikuKiri`))
  (bind _sikukanan_2 (`self.SikuKanan`))
  (bind _kepala (`self.Kepala`))
  (bind _kepala_2 (`self.Kepala`))
  (bind _pahakanan (`self.PahaKanan`))
  (bind _pundakkiri_2 (`self.PundakKiri`))
  (bind _pahakanan_2 (`self.PahaKanan`))
  (bind _pahakiri (`self.PahaKiri`))
  (bind _pahakiri_2 (`self.PahaKiri`))
  (bind _sikukiri_2 (`self.SikuKiri`))
  (bind (_direction _newtrack_0) (`Timeline|Timeline` :!via `PlayFromStart` :!label _label)
    (:`Update`
      (set `self.Alpha` _newtrack_0)
      (`SceneComponent.K2_SetRelativeRotation` _pundakkanan_2 (`KismetMathLibrary.RLerp` (`SceneComponent.RelativeRotation` _pundakkanan_2) (struct :`Roll` 100.0) (`self.Alpha`)) false false)
      (`SceneComponent.K2_SetRelativeRotation` _sikukanan (`KismetMathLibrary.RLerp` (`SceneComponent.RelativeRotation` _sikukanan) (struct :`Roll` 50.0) (`self.Alpha`)) false false)
      (`SceneComponent.K2_SetRelativeRotation` _pundakkiri (`KismetMathLibrary.RLerp` (`SceneComponent.RelativeRotation` _pundakkiri) (struct :`Roll` -60.0) (`self.Alpha`)) false false)
      (`SceneComponent.K2_SetRelativeRotation` _sikukiri (`KismetMathLibrary.RLerp` (`SceneComponent.RelativeRotation` _sikukiri) (struct :`Roll` 50.0) (`self.Alpha`)) false false)
      (`SceneComponent.K2_SetRelativeRotation` _kepala_2 (`KismetMathLibrary.RLerp` (`SceneComponent.RelativeRotation` _kepala_2) (struct :`Roll` -20.0) (`self.Alpha`)) false false)
      (`SceneComponent.K2_SetRelativeRotation` _pahakanan_2 (`KismetMathLibrary.RLerp` (`SceneComponent.RelativeRotation` _pahakanan_2) (struct) (`self.Alpha`)) false false)
      (`SceneComponent.K2_SetRelativeRotation` _pahakiri_2 (`KismetMathLibrary.RLerp` (`SceneComponent.RelativeRotation` _pahakiri_2) (struct :`Roll` -30.0) (`self.Alpha`)) false false))
    (:`Finished`
      (bind (_direction_2 _newtrack_0_2) (`Timeline|Timeline_0` :!via `PlayFromStart`)
        (:`Update`
          (set `self.Alpha` _newtrack_0_2)
          (`SceneComponent.K2_SetRelativeRotation` _pundakkanan (`KismetMathLibrary.RLerp` (`SceneComponent.RelativeRotation` _pundakkanan) (struct :`Roll` 50.0) (`self.Alpha`)) false false)
          (`SceneComponent.K2_SetRelativeRotation` _sikukanan_2 (`KismetMathLibrary.RLerp` (`SceneComponent.RelativeRotation` _sikukanan_2) (struct :`Roll` -50.0) (`self.Alpha`)) false false)
          (`SceneComponent.K2_SetRelativeRotation` _pundakkiri_2 (`KismetMathLibrary.RLerp` (`SceneComponent.RelativeRotation` _pundakkiri_2) (struct :`Roll` -120.0) (`self.Alpha`)) false false)
          (`SceneComponent.K2_SetRelativeRotation` _sikukiri_2 (`KismetMathLibrary.RLerp` (`SceneComponent.RelativeRotation` _sikukiri_2) (struct :`Roll` -50.0) (`self.Alpha`)) false false)
          (`SceneComponent.K2_SetRelativeRotation` _kepala (`KismetMathLibrary.RLerp` (`SceneComponent.RelativeRotation` _kepala) (struct :`Roll` 20.0) (`self.Alpha`)) false false)
          (`SceneComponent.K2_SetRelativeRotation` _pahakanan (`KismetMathLibrary.RLerp` (`SceneComponent.RelativeRotation` _pahakanan) (struct :`Roll` 30.0) (`self.Alpha`)) false false)
          (`SceneComponent.K2_SetRelativeRotation` _pahakiri (`KismetMathLibrary.RLerp` (`SceneComponent.RelativeRotation` _pahakiri) (struct) (`self.Alpha`)) false false))
        (:`Finished`
          (goto _label :!via `PlayFromStart`))))))

(fn `Start`
  (bind _output_get (set `self.ModelComponent` (`|MakeArray` (`self.KakiKiri`) (`self.KakiKanan`) (`self.3`) (`self.4`) (`self.LututKiri`) (`self.LututKanan`) (`self.7`) (`self.8`) (`self.PahaKiri`) (`self.PahaKanan`) (`self.Badan`) (`self.12`) (`self.13`) (`self.14`) (`self.15`) (`self.16`) (`self.17`) (`self.PundakKiri`) (`self.19`) (`self.SikuKiri`) (`self.21`) (`self.TanganKiri`) (`self.PundakKanan`) (`self.24`) (`self.SikuKanan`) (`self.26`) (`self.TanganKanan`) (`self.28`) (`self.Kepala`) (`self.30`) (`self.31`) (`self.32`) (`self.33`) (`self.34`))))
  (for _array_element _output_get
    (`SceneComponent.SetVisibility` _array_element (`self.isModel?`) false))
  (set `self.MainRoot` (`|MakeArray` (`self.Badan`) (`self.Kepala`) (`self.PundakKiri`) (`self.PundakKanan`) (`self.SikuKiri`) (`self.SikuKanan`) (`self.TanganKiri`) (`self.TanganKanan`) (`self.PahaKiri`) (`self.PahaKanan`) (`self.LututKiri`) (`self.LututKanan`) (`self.KakiKiri`) (`self.KakiKanan`)))
  (return))

(fn `UserConstructionScript`
  (`parent.UserConstructionScript`))