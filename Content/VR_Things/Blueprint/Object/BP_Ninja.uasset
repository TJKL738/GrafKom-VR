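; BP_Ninja is a VR object Blueprint for a ninja character built from separate body-part and sword components, with Indonesian names.
; On BeginPlay it runs Start before calling the parent BeginPlay.
; Start sets visibility on every model piece from the IsModel flag, then fills MainRoot with the body, head, limb control and joint components.
; Nothing in this graph reads MainRoot, and Tick and overlap events are disabled.
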(event `self.ReceiveBeginPlay`
  (`self.Start`)
  (`parent.ReceiveBeginPlay`))

(fn `Start`
  (bind _output_get (set `self.ModelComponent` (`|MakeArray` (`self.Sepatu_Ka`) (`self.Sepatu_Ki`) (`self.Kaki_Ka`) (`self.Kaki_Ki`) (`self.PahaBawah_Ka`) (`self.PahaBawah_Ki`) (`self.Lutut_Ka`) (`self.Lutut_Ki`) (`self.PahaAtas_Ka`) (`self.PahaAtas_Ki`) (`self.BadanBawah`) (`self.Perut`) (`self.BadanAtas`) (`self.LenganAtas_Ka`) (`self.LenganBawah_Ka`) (`self.Tangan_Ka`) (`self.UjungTangan_Ka`) (`self.LenganAtas_Ki`) (`self.LenganBawah_Ki`) (`self.Tangan_Ki`) (`self.UjungTangan_Ki`) (`self.SwordHandle_1`) (`self.SwordGuardTengah_1`) (`self.SwordGuardSamping1_1`) (`self.SwordGuardSamping2_1`) (`self.SwordBlade_1`) (`self.Kepala`) (`self.Hidung`) (`self.Mata_Ka`) (`self.GarisMata_Ka`) (`self.Mata_Ki`) (`self.GarisMata_Ki`) (`self.KepalaNinja`) (`self.SwordHandle_2`) (`self.SwordGuardTengah_2`) (`self.SwordGuardSamping1_2`) (`self.SwordGuardSamping2_2`) (`self.SwordBlade_2`) (`self.SwordHandle_3`) (`self.SwordGuardTengah_3`) (`self.SwordGuardSamping1_3`) (`self.SwordGuardSamping2_3`) (`self.SwordBlade_3`))))
  (for _array_element _output_get
    (`SceneComponent.SetVisibility` _array_element (`self.isModel?`) false))
  (set `self.MainRoot` (`|MakeArray` (`self.BadanBawah`) (`self.KontrolKaki_Ki`) (`self.Lutut_Ki`) (`self.EngselKaki_Ki`) (`self.KontrolKaki_Ka`) (`self.Lutut_Ka`) (`self.EngselKaki_Ka`) (`self.BadanAtas`) (`self.Kepala`) (`self.KontrolTangan_Ka`) (`self.Tangan_Ka`) (`self.KontrolTangan_Ki`) (`self.Tangan_Ki`)))
  (return))

(fn `UserConstructionScript`
  (`parent.UserConstructionScript`))