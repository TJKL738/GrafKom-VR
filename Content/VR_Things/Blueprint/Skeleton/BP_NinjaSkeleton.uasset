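; BP_NinjaSkeleton is a child Blueprint that defines the body-part list for a ninja skeleton in the VR content.
; On BeginPlay it fills the Root array with Indonesian-named parts covering lower and upper body, head, and left and right limb controls and joints.
; It then calls the parent BeginPlay, so the inherited logic runs with the array already set.
; Tick, overlap and construction add no logic of their own.
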(event `self.ReceiveBeginPlay`
  (set `self.Root` (`|MakeArray` (`self.BadanBawah`) (`self.KontrolKaki_Ki`) (`self.Lutut_Ki`) (`self.EngselKaki_Ki`) (`self.KontrolKaki_Ka`) (`self.Lutut_Ka`) (`self.EngselKaki_Ka`) (`self.BadanAtas`) (`self.Kepala`) (`self.KontrolTangan_Ka`) (`self.Siku_Ka`) (`self.Tangan_Ka`) (`self.KontrolTangan_Ki`) (`self.Siku_Ki`) (`self.Tangan_Ki`)))
  (`parent.ReceiveBeginPlay`))

(fn `UserConstructionScript`
  (`parent.UserConstructionScript`))