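; VR robot skeleton rig with touchable markers on body joints, used to pick a joint for animation.
; BeginPlay fills Root with joint components and spawns overlap mesh markers at their locations.
; A VR pawn index-finger overlap passes that joint's BP_Root child actor to BP_MejaAnimasi as Seq and makes its marker blink.
; The Animation event applies each BP_Root's stored rotation at the current Index to BP_Robot's MainRoot parts.
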(event `self.ReceiveBeginPlay`
  (set `self.Root` (`|MakeArray` (`self.Badan`) (`self.Kepala`) (`self.PundakKiri`) (`self.PundakKanan`) (`self.SikuKiri`) (`self.SikuKanan`) (`self.TanganKiri`) (`self.TanganKanan`) (`self.PahaKiri`) (`self.PahaKanan`) (`self.LututKiri`) (`self.LututKanan`) (`self.KakiKiri`) (`self.KakiKanan`)))
  (`self.SpawnTitikInteract`
    (:`Out`
      (for _array_element (`self.AllOverlap`)
        (add `PrimitiveComponent.OnComponentBeginOverlap` _array_element (delegate `Overlaped`)))
      (`self.SendDataToMejaAnimasi` (`|GetArrayItem` (`self.AllOverlap`))))))

(event `Overlaped`
  (params (OverlappedComponent :type "PrimitiveComponent Object Reference") (OtherActor :type "Actor Object Reference") (OtherComp :type "PrimitiveComponent Object Reference") (OtherBodyIndex :type Integer) (bFromSweep :type Boolean) (SweepResult :type "HitResult Structure (by ref)"))
  (bind _asvrpawn_manual (cast `/Game/VR_Things/Blueprint/BP_GameThings/VRPawnManual` OtherActor))
  (if (or (== (`/Game/VR_Things/Blueprint/BP_GameThings/VRPawnManual.IndexLeft` _asvrpawn_manual) OtherComp) (== (`/Game/VR_Things/Blueprint/BP_GameThings/VRPawnManual.IndexRight` _asvrpawn_manual) OtherComp))
    (`self.SendDataToMejaAnimasi` OverlappedComponent)))

(event `Animation`
  (bind _returnvalue (`GameplayStatics.GetActorOfClass` "/Game/VR_Things/Blueprint/Object/BP_Robot.BP_Robot_C"))
  (for (_array_element _array_index) (`/Game/VR_Things/Blueprint/Object/BP_Robot.MainRoot` _returnvalue)
    (bind _asbp_root (cast `/Game/VR_Things/Blueprint/Skeleton/BP_Root` (`ChildActorComponent.ChildActor` (`|GetArrayItem` (`self.Root`) _array_index))))
    (`SceneComponent.K2_SetRelativeRotation` _array_element (`|GetArrayItem` (`/Game/VR_Things/Blueprint/Skeleton/BP_Root.Rot` _asbp_root) (`self.Index`)) false false)))

(fn `UserConstructionScript`)