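; BP_SkeletonRobot is a child Blueprint for a robot skeleton in the VR content.
; On BeginPlay it fills the Root array with fourteen Indonesian-named body parts: body, head, and left/right shoulders, elbows, hands, thighs, knees and feet.
; It then calls the parent BeginPlay, so the array is set before any parent logic runs.
; Tick and overlap events are unused, and the construction script only calls its parent.
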(event `self.ReceiveBeginPlay`
  (set `self.Root` (`|MakeArray` (`self.Badan`) (`self.Kepala`) (`self.PundakKiri`) (`self.PundakKanan`) (`self.SikuKiri`) (`self.SikuKanan`) (`self.TanganKiri`) (`self.TanganKanan`) (`self.PahaKiri`) (`self.PahaKanan`) (`self.LututKiri`) (`self.LututKanan`) (`self.KakiKiri`) (`self.KakiKanan`)))
  (`parent.ReceiveBeginPlay`))

(fn `UserConstructionScript`
  (`parent.UserConstructionScript`))