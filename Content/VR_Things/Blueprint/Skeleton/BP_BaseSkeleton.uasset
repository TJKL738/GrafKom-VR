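; BP_BaseSkeleton is a VR skeleton rig for selecting joints and playing pose animation on BP_BaseModel.
; It spawns overlap meshes from its Root child actors; a pawn index-finger touch makes one blink and passes its BP_Root to BP_MejaAnimasi as Seq.
; Animation applies the current indexed rotation from each BP_Root to the model's MainRoot parts.
; PlayA chains five timeline passes, lerping between successive stored rotations.
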(event `self.ReceiveBeginPlay`
  (`self.SpawnTitikInteract`
    (:`Out`
      (for _array_element (`self.AllOverlap`)
        (add `PrimitiveComponent.OnComponentBeginOverlap` _array_element (delegate `Overlaped`)))
      (`self.SendDataToMejaAnimasi` (`|GetArrayItem` (`self.AllOverlap`))))))

(event `Overlaped`
  (params (OverlappedComponent :type "PrimitiveComponent Object Reference") (OtherActor :type "Actor Object Reference") (OtherComp :type "PrimitiveComponent Object Reference") (OtherBodyIndex :type Integer) (bFromSweep :type Boolean) (SweepResult :type "HitResult Structure (by ref)"))
  (bind _asvrpawn_manual (cast `/Game/VR_Things/Blueprint/BP_GameThings/VRPawnManual` OtherActor))
  (if (or (== (`/Game/VR_Things/Blueprint/BP_GameThings/VRPawnManual.IndexLeft` _asvrpawn_manual) OtherComp) (== (`/Game/VR_Things/Blueprint/BP_GameThings/VRPawnManual.IndexRight` _asvrpawn_manual) OtherComp))
    (`self.SendDataToMejaAnimasi` OverlappedComponent)))

(event `Animation`
  (bind _returnvalue (`GameplayStatics.GetActorOfClass` "/Game/VR_Things/Blueprint/Object/BP_BaseModel.BP_BaseModel_C"))
  (for (_array_element _array_index) (`/Game/VR_Things/Blueprint/Object/BP_BaseModel.MainRoot` _returnvalue)
    (bind _asbp_root (cast `/Game/VR_Things/Blueprint/Skeleton/BP_Root` (`ChildActorComponent.ChildActor` (`|GetArrayItem` (`self.Root`) _array_index))))
    (`SceneComponent.K2_SetRelativeRotation` _array_element (`|GetArrayItem` (`/Game/VR_Things/Blueprint/Skeleton/BP_Root.Rot` _asbp_root) (`self.Index`)) false false)))

(event `PlayA`
  (bind _index (`self.Index`))
  (set `self.Index` 0)
  (bind _returnvalue (`GameplayStatics.GetActorOfClass` "/Game/VR_Things/Blueprint/Object/BP_BaseModel.BP_BaseModel_C" :!label _label))
  (bind (_direction _newtrack_0) (`Timeline|Timeline` :!via `PlayFromStart`)
    (:`Update`
      (for (_array_element _array_index) (`/Game/VR_Things/Blueprint/Object/BP_BaseModel.MainRoot` _returnvalue)
        (bind _asbp_root (cast `/Game/VR_Things/Blueprint/Skeleton/BP_Root` (`ChildActorComponent.ChildActor` (`|GetArrayItem` (`self.Root`) _array_index))))
        (if (!= _index 0)
          (bind _rot (`/Game/VR_Things/Blueprint/Skeleton/BP_Root.Rot` _asbp_root))
          (bind _output (`|GetArrayItem` _rot _index))
          (`SceneComponent.K2_SetRelativeRotation` _array_element (`KismetMathLibrary.RLerp` (`|GetArrayItem` _rot (- _index 1)) _output _newtrack_0) false false)
          (else
            (`SceneComponent.K2_SetRelativeRotation` _array_element (`KismetMathLibrary.RLerp` (struct) _output _newtrack_0) false false)))))
    (:`Finished`
      (set `self.Index` (+ (`self.Index`) 1))
      (if (!= (`self.Index`) 5)
        (goto _label)))))

(fn `UserConstructionScript`)